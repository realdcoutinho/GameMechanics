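; Base weapon Blueprint that handles primary and secondary fire input through start/stop events.
; Starting primary fire spawns a projectile at the FireSocket transform, then repeats on a looping timer at an interval set by PrimaryFireRate.
; A DoOnce prevents stacked timers; stopping clears the timer by function name and resets the gate.
; Secondary fire is a stub that only prints a debug string.
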(event `FirePrimary`
  (params (`Is Start` :type Boolean :default true))
  (if `Is Start`
    (`/Engine/EditorBlueprintResources/StandardMacros.DoOnce` false :!label _label
      (:`Completed`
        (`self.SpawnPrimaryProjectile`)
        (`KismetSystemLibrary.K2_SetTimerDelegate` (delegate `SpawnPrimaryProjectile`) (/ 1.0 (`self.PrimaryFireRate`)) true)))
    (else
      (`KismetSystemLibrary.K2_ClearTimer` null "SpawnPrimaryProjectile")
      (goto _label :!via `Reset`))))

(event `SpawnPrimaryProjectile`
  (`|SpawnActorFromClass` (`self.PrimaryProjectileClass`) (`SceneComponent.K2_GetComponentToWorld` (`self.FireSocket`)) "Undefined" "OverrideRootScale" null null)
  (`KismetSystemLibrary.PrintString` "FirePrimary"))

(event `FireSecundary`
  (params (`Is Start` :type Boolean :default true))
  (if `Is Start`
    (`KismetSystemLibrary.PrintString` "FireSecundary" true true (struct :`R` 1.0 :`B` 0.60955 :`A` 1.0))))

(fn `UserConstructionScript`)