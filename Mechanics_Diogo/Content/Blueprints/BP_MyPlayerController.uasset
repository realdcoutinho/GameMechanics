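; Player controller that handles world-axis movement, aiming and firing for the controlled pawn, in a top-down style.
; Primary and secondary fire presses and releases pass to BP_PlayerCharacter as true or false.
; Mouse movement traces under the cursor and sets control yaw toward the hit point.
; LookUp and LookRight axes set control rotation from their input vector, with both aiming paths ignoring input below a small threshold.
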(event `InputAxis|MovementFoward`
  (params (AxisValue :type "Float (single-precision)"))
  ;[1 1 1] Handle Movement Input
  (`Pawn.AddMovementInput` (`self.K2_GetPawn`) (1.0 0.0 0.0) AxisValue false))

(event `InputAction|FirePrimary`
  (params (Key :type "Key Structure"))
  (bind _returnvalue (`self.K2_GetPawn`))
  ;[1 1 1] Fire
  (:`Pressed`
    (bind _asbp_player_character (cast `/Game/Blueprints/BP_PlayerCharacter` _returnvalue))
    (`/Game/Blueprints/BP_PlayerCharacter.PrimaryFire` _asbp_player_character true))
  (:`Released`
    (bind _asbp_player_character_2 (cast `/Game/Blueprints/BP_PlayerCharacter` _returnvalue))
    (`/Game/Blueprints/BP_PlayerCharacter.PrimaryFire` _asbp_player_character_2 false)))

(event `InputAxis|MovementRight`
  (params (AxisValue :type "Float (single-precision)"))
  ;[1 1 1] Handle Movement Input
  (`Pawn.AddMovementInput` (`self.K2_GetPawn`) (0.0 1.0 0.0) AxisValue false))

(event `InputAction|FireSecundary`
  (params (Key :type "Key Structure"))
  (bind _returnvalue (`self.K2_GetPawn`))
  ;[1 1 1] Fire
  (:`Pressed`
    (bind _asbp_player_character (cast `/Game/Blueprints/BP_PlayerCharacter` _returnvalue))
    (`/Game/Blueprints/BP_PlayerCharacter.SecundaryFire` _asbp_player_character true))
  (:`Released`
    (bind _asbp_player_character_2 (cast `/Game/Blueprints/BP_PlayerCharacter` _returnvalue))
    (`/Game/Blueprints/BP_PlayerCharacter.SecundaryFire` _asbp_player_character_2 false)))

(event `self.ReceiveTick`
  (params (DeltaSeconds :type "Float (single-precision)")))

(event `InputAxisKey|MouseX`
  (params (AxisValue :type "Float (single-precision)"))
  (bind (_hitresult _returnvalue) (`self.GetHitResultUnderCursorByChannel` "TraceTypeQuery1"))
  (bind (_returnvalue_roll _returnvalue_pitch _returnvalue_yaw) (`KismetMathLibrary.BreakRotator` (`KismetMathLibrary.FindLookAtRotation` (`self.K2_GetActorLocation` (`self.K2_GetPawn`)) (`.Location` (`GameplayStatics.BreakHitResult` _hitresult)))))
  ;[1 1 1] Aiming
  (if (> (`KismetMathLibrary.VSize` (`KismetMathLibrary.MakeVector` AxisValue (stale `InputAxisKey|MouseY` AxisValue))) 0.25) :!label _label
    (if _returnvalue
      (`self.SetControlRotation` (`KismetMathLibrary.MakeRotator` 0.0 0.0 _returnvalue_yaw)))))

(event `InputAxisKey|MouseY`
  (params (AxisValue :type "Float (single-precision)"))
  ;[1 1 1] Aiming
  (goto _label))

(event `InputAxis|LookUp`
  (params (AxisValue :type "Float (single-precision)"))
  ;[1 1 1] rotation. turn off bp_player character check orient to chacnge to aim
  (`|ExecutionSequence` :!label _label_2
    (:`then_2`
      (bind _returnvalue (`KismetMathLibrary.MakeVector` AxisValue (stale `InputAxis|LookRight` AxisValue)))
      (if (> (`KismetMathLibrary.VSize` _returnvalue) 0.25)
        (`self.SetControlRotation` (`KismetMathLibrary.Conv_VectorToRotator` _returnvalue))))))

(event `InputAxis|LookRight`
  (params (AxisValue :type "Float (single-precision)"))
  ;[1 1 1] rotation. turn off bp_player character check orient to chacnge to aim
  (goto _label_2))

(fn `UserConstructionScript`)