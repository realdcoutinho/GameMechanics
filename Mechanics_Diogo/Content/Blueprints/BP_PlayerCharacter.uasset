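; Player character Blueprint that equips a weapon and relays fire input to it.
; On BeginPlay it spawns a BP_BaseWeapon at the GunSocket component, stores it as CurrentWeapon and attaches it there.
; PrimaryFire and SecundaryFire events check that the weapon is valid, then forward their start flag to its matching fire functions.
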(event `self.ReceiveBeginPlay`
  (bind _gunsocket (`self.GunSocket`))
  (`parent.ReceiveBeginPlay`)
  ;[1 1 1] Weapon Spawn
  (bind _returnvalue (`|SpawnActorFromClass` "/Game/Blueprints/BP_BaseWeapon.BP_BaseWeapon_C" (`SceneComponent.K2_GetComponentToWorld` _gunsocket) "Undefined" "OverrideRootScale" null null))
  (bind _output_get (set `self.CurrentWeapon` _returnvalue))
  (`self.K2_AttachToComponent` _output_get _gunsocket "None" "SnapToTarget" "SnapToTarget" "KeepRelative" true))

(event `PrimaryFire`
  (params (`Is Start` :type Boolean :default true))
  (bind _currentweapon (`self.CurrentWeapon`)
    (:`then`
      (`/Game/Blueprints/BP_BaseWeapon.FirePrimary` _currentweapon `Is Start`))
    (:`else`)))

(event `SecundaryFire`
  (params (`Is Start` :type Boolean :default true))
  (bind _currentweapon (`self.CurrentWeapon`)
    (:`then`
      (`/Game/Blueprints/BP_BaseWeapon.FireSecundary` _currentweapon `Is Start`))
    (:`else`)))

(fn `UserConstructionScript`
  (`parent.UserConstructionScript`))