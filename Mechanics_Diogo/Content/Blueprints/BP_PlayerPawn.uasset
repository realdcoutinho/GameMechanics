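; BP_PlayerPawn is a player pawn that moves from movement input and turns to face its direction of travel.
; Each tick it consumes the input vector, clamps it to unit length, scales it by speed and delta time, and applies a swept world offset.
; When there is movement it updates a desired rotation, and the actor continually lerps toward it along the shortest path.
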(event `self.ReceiveTick`
  (params (DeltaSeconds :type "Float (single-precision)"))
  ;[1 1 1] Movement
  (bind _returnvalue (`self.ConsumeMovementInputVector`))
  (bind _returnvalue_2 (* (* (`KismetMathLibrary.ClampVectorSize` _returnvalue 0.0 1.0) DeltaSeconds) (`self.MovementSpeed`)))
  (`self.K2_AddActorWorldOffset` _returnvalue_2 true)
  ;[1 1 1] Is there movement input?
  (if (> (`KismetMathLibrary.VSizeSquared` _returnvalue_2) 0.0)
    (set `self.DesiredRotation` (`KismetMathLibrary.Conv_VectorToRotator` _returnvalue_2)))
  (`self.K2_SetActorRotation` (`KismetMathLibrary.RLerp` (`self.K2_GetActorRotation`) (`self.DesiredRotation`) (* DeltaSeconds (`self.RotationSpeed`)) true)))

(fn `UserConstructionScript`)